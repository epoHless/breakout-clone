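; BP_Ball is a brick-breaker ball that bounces off whatever it hits and scores against bricks.
; On hit, a brick adds score, spawns its PP and shrinks, while a killzone only prints a loss message.
; Every hit also mirrors velocity about the impact normal at the same speed, then zeroes X to keep motion in the YZ plane.
; Any overlap on the sphere destroys the ball.
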(event `self.Sphere.OnComponentHit`
  (params (HitComponent :type "PrimitiveComponent Object Reference") (OtherActor :type "Actor Object Reference") (OtherComp :type "PrimitiveComponent Object Reference") (NormalImpulse :type "Vector Structure") (Hit :type "HitResult Structure (by ref)"))
  (bind _returnvalue (`self.GetVelocity`))
  (`|ExecutionSequence`
    (:`then_0`
      (cast `/Game/Blueprints/BP_Killzone` OtherActor)
      (`KismetSystemLibrary.PrintString` "YOU LOST"))
    (:`then_1`
      (bind _asbp_brick (cast `/Game/Blueprints/BP_Brick` OtherActor)
        (:`then`
          (`/Game/Blueprints/ScoreLibrary.Add Score` _asbp_brick)
          (`/Game/Blueprints/BP_Brick.Spawn PP` _asbp_brick)
          (`/Game/Blueprints/BP_Brick.Shrink` _asbp_brick))
        (:`CastFailed`
          _))
      (set `MovementComponent.Velocity` (`KismetMathLibrary.MakeVector` 0.0 (.y (* (`KismetMathLibrary.GetReflectionVector` (`KismetMathLibrary.Normal` _returnvalue) Hit_ImpactNormal) (`KismetMathLibrary.VSize` _returnvalue))) (.z (* (`KismetMathLibrary.GetReflectionVector` (`KismetMathLibrary.Normal` _returnvalue) Hit_ImpactNormal) (`KismetMathLibrary.VSize` _returnvalue)))) (`self.ProjectileMovement`)))))

(event `self.Sphere.OnComponentBeginOverlap`
  (params (OverlappedComponent :type "PrimitiveComponent Object Reference") (OtherActor :type "Actor Object Reference") (OtherComp :type "PrimitiveComponent Object Reference") (OtherBodyIndex :type Integer) (bFromSweep :type Boolean) (SweepResult :type "HitResult Structure (by ref)"))
  (`self.K2_DestroyActor`))

(fn `UserConstructionScript`)