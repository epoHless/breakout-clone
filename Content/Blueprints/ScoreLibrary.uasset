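; ScoreLibrary holds an Add Score function that handles scoring and the win check for a brick-breaking game.
; It casts the game mode to GM_Base and decrements its remaining brick count.
; While bricks remain, it adds the brick's Value to the current score and prints score and bricks left.
; At zero or below it only prints a win message, without adding that last brick's value.
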(fn `Add Score`
  (params (Brick :type "/Game/Blueprints/BP_Brick Object Reference"))
  (bind _asgm_base (cast `/Game/Gamemode/GM_Base` (`GameplayStatics.GetGameMode` null)))
  (bind _result (`/Engine/EditorBlueprintResources/StandardMacros.DecrementInt` (`/Game/Gamemode/GM_Base.Total Bricks` _asgm_base))
    (:`  `
      (if (> _result 0)
        (bind _output_get (set `/Game/Gamemode/GM_Base.Current Score` (+ (`/Game/Gamemode/GM_Base.Current Score` _asgm_base) (`/Game/Blueprints/BP_Brick.Value` Brick)) _asgm_base))
        (`KismetSystemLibrary.PrintString` null (`KismetStringLibrary.Concat_StrStr` "Current Score : " (`KismetStringLibrary.Conv_IntToString` _output_get) " | Bricks Left : " (`KismetStringLibrary.Conv_IntToString` _result)))
        (else
          (`KismetSystemLibrary.PrintString` null "You Won!"))))))