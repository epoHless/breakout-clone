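; BP_Brick is a breakable brick actor that shrinks away when hit and can drop a power-up.
; Shrink disables the cube's collision, then plays a timeline that eases the actor's scale from full size before destroying it.
; SpawnPP rolls against SpawnProb to spawn a PowerUp at the brick's transform.
; The construction script creates a dynamic material instance of M_Brick tinted by the Color variable.
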(event `Shrink`
  ;[1 1 1] Shrink a brick when hit
  (`PrimitiveComponent.SetCollisionEnabled` (`self.Cube`) "NoCollision")
  (bind (_direction _value) (`Timeline|Scale` :!via `PlayFromStart`)
    (:`Update`
      (`self.SetActorScale3D` (`|EaseFunction` "EaseInOut" _value (1.0 1.0 1.0))))
    (:`Finished`
      (`self.K2_DestroyActor`))))

(event `Spawn PP`
  (if (<= (`KismetMathLibrary.RandomFloatInRange` 0.0 1.0) (`self.Spawn Prob`))
    (`|SpawnActorFromClass` "/Game/Blueprints/PowerUp.PowerUp_C" (`self.GetTransform`) "Undefined" "OverrideRootScale" null null)))

(fn `UserConstructionScript`
  (bind _returnvalue (`PrimitiveComponent.CreateDynamicMaterialInstance` (`self.Cube`) 0 "/Game/Materials/M_Brick.M_Brick" "None"))
  (bind _output_get (set `self.Mat` _returnvalue))
  (`MaterialInstanceDynamic.SetVectorParameterValue` _output_get "Color" (`self.Color`)))